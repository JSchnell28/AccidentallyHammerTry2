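; DamageFieldWeapon_BP is a Chaos field actor that breaks and blasts destructible geometry within a sphere when play begins for it.
; On BeginPlay it applies an external cluster strain with no falloff inside the sphere to fracture clusters.
; It then applies a linear velocity from a radial vector scaled by ForceMagnitude, multiplied by a linear radial falloff, pushing pieces outward from the sphere's center.
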(event EventBeginPlay
  (bind _sphere (Variables|Default|GetSphere))
  (Class|FieldSystemComponent|ApplyPhysicsField (Variables|Field|GetFieldSystemComponent) true "Field_ExternalClusterStrain" 0 (Field|SetRadialFalloff (Variables|Default|GetRadialFalloff) 5e+03 0.0 1.0 0.0 (Variables|/Script/Engine.SphereComponent|GetSphereRadius (Variables|Default|GetSphere)) (Transformation|GetWorldLocation (Variables|Default|GetSphere)) "Field_FallOff_None"))
  (Class|FieldSystemComponent|ApplyPhysicsField (Variables|Field|GetFieldSystemComponent) true "Field_LinearVelocity" 0 (Field|SetOperatorField (Variables|Default|GetOperatorField) 1.0 (Field|SetRadialFalloff (Variables|Default|GetRadialFalloff) 1.0 0.0 1.0 0.0 (Variables|/Script/Engine.SphereComponent|GetSphereRadius _sphere) (Transformation|GetWorldLocation _sphere) "Field_Falloff_Linear") (Field|SetRadialVector (Variables|Default|GetRadialVector) (Variables|Default|GetForceMagnitude) (Transformation|GetWorldLocation (Variables|Default|GetSphere))) "Field_Multiply")))

(fn ConstructionScript)