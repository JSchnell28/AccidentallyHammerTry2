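; Character Blueprint that triggers a field system when it touches Chaos Geometry Collection actors.
; When the capsule begins overlapping a Geometry Collection actor, it spawns a FieldSystem actor at that actor's transform.
; The construction script caches one level Geometry Collection actor, but only disconnected collision-binding and kinematic-field nodes use it, and the collision event is empty.
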(event OnComponentBeginOverlap(CapsuleComponent)
  (params (OverlappedComponent :type Primitive%20Component%20Object%20Reference) (OtherActor :type Actor%20Object%20Reference) (OtherComp :type Primitive%20Component%20Object%20Reference) (OtherBodyIndex :type Integer) (bFromSweep :type Boolean) (SweepResult :type Hit%20Result%20Structure%20%28by%20ref%29))
  (bind _asgeometry_collection_actor (Utilities|Casting|CastToGeometryCollectionActor OtherActor))
  (Game|SpawnActorfromClass "/Game/AccidentallyHammerFiles/FieldSystem.FieldSystem_C" (Transformation|GetActorTransform _asgeometry_collection_actor) "Undefined" 0 0))

(event Custom|OnChaosPhysicsCollsion_Event_1
  (params (CollisionInfo :type Chaos%20Physics%20Collision%20Info%20Structure%20%28by%20ref%29)))

(event EventBeginPlay)

(fn ConstructionScript
  (bind _returnvalue (Actor|GetActorOfClass "/Script/GeometryCollectionEngine.GeometryCollectionActor"))
  (Variables|Default|SetGeometryCollectionActor _returnvalue))