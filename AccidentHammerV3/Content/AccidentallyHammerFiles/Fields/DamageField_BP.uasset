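; Damage field actor that breaks Chaos destructible geometry within a spherical area.
; On BeginPlay it waits a configurable delay, then applies a single external cluster strain physics field.
; The strain comes from a radial falloff node centered on the Sphere component, using its radius with no falloff, so the magnitude is uniform throughout the sphere.
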(event EventBeginPlay
  (Utilities|FlowControl|Delay (Variables|Default|GetDelayBeforeDamage))
  (Class|FieldSystemComponent|ApplyPhysicsField (Variables|Field|GetFieldSystemComponent) true "Field_ExternalClusterStrain" 0 (Field|SetRadialFalloff (Variables|Default|GetRadialFalloff) (Variables|Default|GetMagnitude) 0.0 1.0 0.0 (Variables|/Script/Engine.SphereComponent|GetSphereRadius (Variables|Default|GetSphere)) (Transformation|GetWorldLocation (Variables|Default|GetSphere)) "Field_FallOff_None")))

(fn ConstructionScript)